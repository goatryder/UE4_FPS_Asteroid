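; Laser weapon Blueprint that implements the cosmetic sound and particle responses to firing events, with energy drained and restored hooks left empty.
; Fire start and end toggle muzzle particles and a fading fire loop, with a one-shot start effect.
; While firing, the impact sound fades in or out based on whether the last trace hit.
; Hit emitters are capped through a wrap-around index that replaces older ones, and are destroyed when finished.
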(event Custom|OnEmitterFinishPlay
  (params (PSystem :type Particle%20System%20Component%20Object%20Reference))
  ;[1 1 1] Hit FX
  ;;[1 1 1] Spawn hit emitter, limit max hit emitters for current weapon instance
  ;;;[1 1 1] on emitter finished - destroy
  (Utilities|Array|RemoveItem (Variables|HitFX|GetSpawnedHitEffects) PSystem)
  (Components|DestroyComponent PSystem))

(event EventOnPlayEndFireEffects
  (Components|Activation|Deactivate (Variables|Default|GetMuzzleParticle))
  (Audio|Components|Audio|FadeOut (Variables|Default|GetFireSound) 0.2 0.0 "Linear" :!class /Script/Engine.AudioComponent)
  (Audio|Components|Audio|FadeOut (Variables|Default|GetBeamImpactSound) 0.1 0.0 "Linear" :!class /Script/Engine.AudioComponent))

(event EventOnPlayEnergyDrainedEffects)

(event EventOnPlayEnergyRestoredEffects)

(event EventOnPlayHitEffects
  (bind _spawnedhiteffects (Variables|HitFX|GetSpawnedHitEffects))
  (bind _lasthit (Variables|Default|GetLastHit))
  ;[1 1 1] Hit FX
  ;;[1 1 1] Spawn hit emitter, limit max hit emitters for current weapon instance
  (bind _returnvalue (Effects|SpawnEmitteratLocation (Variables|HitFX|GetHitEffect) (.location _lasthit) (Math|Rotator|FindLookatRotation (.location _lasthit) (.tracestart _lasthit)) "0.200000,0.200000,0.200000" false))
  (Utilities|FlowControl|Sequence
    (:then_0
      ;;;[1 1 1] on emitter finished - destroy
      (EventDispatchers|BindEventtoOnSystemFinished _returnvalue (delegate Custom|OnEmitterFinishPlay)))
    (:then_1
      ;;;[1 1 1] Destroy oldest emitter comp in list if exists
      (if (Utilities|Array|IsValidIndex _spawnedhiteffects (Variables|HitFX|GetSpawnedHitEffectIndex))
        (Components|DestroyComponent (Utilities|Array|Get(acopy) _spawnedhiteffects (Variables|HitFX|GetSpawnedHitEffectIndex)))
        (Utilities|Array|RemoveIndex _spawnedhiteffects (Variables|HitFX|GetSpawnedHitEffectIndex))))
    (:then_2
      ;;;[1 1 1] add emitter comp to list
      (Utilities|Array|Insert (Variables|HitFX|GetSpawnedHitEffects) _returnvalue (Variables|HitFX|GetSpawnedHitEffectIndex))
      ;;;[1 1 1] Update next instert index
      (Variables|HitFX|SetSpawnedHitEffectIndex (Math|Integer|%(Integer) (+ (Variables|HitFX|GetSpawnedHitEffectIndex) 1) (Variables|HitFX|GetMaxHitEffectNum))))))

(event EventOnPlayStartFireEffects
  (|StartFireFX)
  (Components|Activation|Activate (Variables|Default|GetMuzzleParticle) false)
  (Audio|Components|Audio|FadeIn (Variables|Default|GetFireSound) 0.1 1.0 0.0 "Linear" :!class /Script/Engine.AudioComponent))

(event EventOnPlayFireEffects
  (bind _lasthit (Variables|Default|GetLastHit))
  (bind _beamimpactsound (Variables|Default|GetBeamImpactSound))
  ;[1 1 1] HandleContinious Fire effect
  (if (.bblockinghit _lasthit)
    (Utilities|IsPlaying _beamimpactsound
      (:false
        (Audio|Components|Audio|FadeIn _beamimpactsound 1.0 1.0 0.5 "Linear" :!class /Script/Engine.AudioComponent)
        (Transformation|SetWorldLocation _beamimpactsound (.location _lasthit) false false)))
    (else
      (Utilities|IsPlaying _beamimpactsound
        (:true
          (Audio|Components|Audio|FadeOut _beamimpactsound 0.2 0.0 "Linear" :!class /Script/Engine.AudioComponent))))))

(fn ConstructionScript)