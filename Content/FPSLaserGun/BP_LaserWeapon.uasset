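; Laser gun weapon Blueprint that supplies the audio and visual feedback for firing, hits and energy drain or restore events.
; Start and end fire events toggle muzzle and beam particles, looping sounds and the player's camera shake.
; Tick aims the beam at the attached character's view point, falling back to the last trace end.
; Impact sound fades with blocking hits, while a ring-indexed array caps hit emitters by destroying the oldest.
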(event EventOnPlayEndFireEffects
  (|Fadeoutfiresounds,deactivateparticles)
  (|LegacyCameraShakeEnd))

(event EventTick
  (params (DeltaSeconds :type Float%20%28single-precision%29))
  (|CalculateBeamTargetPoint))

(event EventOnPlayEnergyDrainedEffects
  (Audio|PlaySound2D "/Game/FPSLaserGun/Audio/CompileFailed.CompileFailed" 1.0 1.0 0.0 0 0))

(event EventOnPlayEnergyRestoredEffects
  (Audio|PlaySound2D "/Game/FPSLaserGun/Audio/CompileSuccess.CompileSuccess" 1.0 1.0 0.0 0 0))

(event EventOnPlayHitEffects
  (|Spawnhitemitter,limitmaxhitemittersforcurrentweaponinstance))

(event EventOnPlayStartFireEffects
  (|PlayStartFire3DSoundandspawnshortStartFireEffect)
  (|Fadeinfiresounds,activateparticles)
  (|LegacyCameraShakeStart))

(event EventOnPlayFireEffects
  (|HandleContiniousFire3DSoundeffect))

(fn ConstructionScript
  (Components|Activation|SetAutoActivate (Variables|Default|GetBeamPSC) false))

(event Custom|OnEmitterFinishPlay
  (params (PSystem :type Particle%20System%20Component%20Object%20Reference))
  ;[1 1 1] on emitter finished - destroy
  (Utilities|Array|RemoveItem (Variables|HitFX|GetSpawnedHitEffects) PSystem)
  (Components|DestroyComponent PSystem))