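; BP_ShootDummy is a target dummy that tallies the damage it receives, apparently for testing the FPS laser gun.
; On BeginPlay it binds to its own OnTakeAnyDamage event, adding each hit to a running total.
; Every tick it draws that total as a purple debug string at the DbgTextLocation component's world position.
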(event Custom|OnTakeAnyDamage_Event_0
  (params (DamagedActor :type Actor%20Object%20Reference) (Damage :type Float%20%28single-precision%29) (DamageType :type Damage%20Type%20Object%20Reference) (InstigatedBy :type Controller%20Object%20Reference) (DamageCauser :type Actor%20Object%20Reference))
  (Variables|Default|SetDamgeRecieved (+ Damage (Variables|Default|GetDamgeRecieved))))

(event EventBeginPlay
  (EventDispatchers|AssignOnTakeAnyDamage (delegate Custom|OnTakeAnyDamage_Event_0)))

(event EventTick
  (params (DeltaSeconds :type Float%20%28single-precision%29))
  (Rendering|Debug|DrawDebugString (Transformation|GetWorldLocation (Variables|Default|GetDbgTextLocation)) (Utilities|String|Append "Damage Recieved: " (Utilities|String|ToString(Text) (Utilities|Text|ToText(Float) (Variables|Default|GetDamgeRecieved) "HalfToEven" false true 1 324 1 1))) 0 "(R=0.633940,G=0.090332,B=0.963542,A=1.000000)"))

(fn ConstructionScript)