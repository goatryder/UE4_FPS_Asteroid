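; BP_ShootDummy is a target dummy for testing weapon damage, showing its state as on-screen debug text.
; Any damage it takes adds to a running total and lowers a health value clamped between zero and its initial value.
; Lost health becomes a 0-1 alpha that drives the LaserAlpha parameter of a dynamic material created on the mesh in the construction script.
; Tick draws total damage, health and alpha at a text anchor component.
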(event Custom|OnTakeAnyDamage_Event_0
  (params (DamagedActor :type Actor%20Object%20Reference) (Damage :type Float%20%28single-precision%29) (DamageType :type Damage%20Type%20Object%20Reference) (InstigatedBy :type Controller%20Object%20Reference) (DamageCauser :type Actor%20Object%20Reference))
  (bind _dynmaterial (Variables|Default|GetDynMaterial))
  (Variables|Default|SetDamgeRecieved (+ Damage (Variables|Default|GetDamgeRecieved)))
  (Variables|Default|SetHealth (Math|Float|Clamp(Float) (- (Variables|Default|GetHealth) Damage) 0.0 (Variables|Default|GetInitialHealth)))
  (Variables|Default|SetHealthAlpha (- 1.0 (Math|Float|Clamp(Float) (/ (Variables|Default|GetHealth) (Variables|Default|GetInitialHealth)))))
  (Utilities|IsValid _dynmaterial
    (:Is%20Valid
      (Rendering|Material|SetScalarParameterValue _dynmaterial "LaserAlpha" (Variables|Default|GetHealthAlpha) :!class /Script/Engine.MaterialInstanceDynamic))))

(event EventBeginPlay
  (EventDispatchers|AssignOnTakeAnyDamage (delegate Custom|OnTakeAnyDamage_Event_0)))

(event EventTick
  (params (DeltaSeconds :type Float%20%28single-precision%29))
  (Rendering|Debug|DrawDebugString (Transformation|GetWorldLocation (Variables|Default|GetDbgTextLocation)) (Utilities|String|Append "Damage Recieved: " (Utilities|String|ToString(Text) (Utilities|Text|ToText(Float) (Variables|Default|GetDamgeRecieved) "HalfToEven" false true 1 324 1 1)) " 
Health:" (Utilities|String|ToString(Text) (Utilities|Text|ToText(Float) (Variables|Default|GetHealth) "HalfToEven" false true 1 324 1 1)) " 
Alpha:" (Utilities|String|ToString(Text) (Utilities|Text|ToText(Float) (Variables|Default|GetHealthAlpha) "HalfToEven" false true 1 324 1 1))) 0 "(R=1.000000,G=1.000000,B=1.000000,A=1.000000)"))

(fn ConstructionScript
  (bind _staticmesh (Variables|Default|GetStaticMesh))
  (bind _returnvalue (Rendering|Material|CreateDynamicMaterialInstance _staticmesh 0 (Rendering|Material|GetMaterial _staticmesh 0) "None" :!class /Script/Engine.PrimitiveComponent))
  (Variables|Default|SetDynMaterial _returnvalue)
  (Rendering|Material|SetMaterial _staticmesh 0 _returnvalue))